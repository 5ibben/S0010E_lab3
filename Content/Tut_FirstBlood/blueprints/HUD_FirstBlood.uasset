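; HUD_FirstBlood is a HUD Blueprint that draws a full-screen material and a coin counter for the side-scroller player.
; Each DrawHUD call picks one of three materials from the Blue, Green and Red mode flags, checked in that order, and sets BlueMode when none is on.
; It then draws a coin icon and the SideScrollerCharacter's Coins count near the top-right corner, positioned relative to screen width.
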(event EventBeginPlay)

(event Collision|EventActorBeginOverlap
  (params (OtherActor :type Actor%20Object%20Reference)))

(event EventTick
  (params (DeltaSeconds :type Float%20%28single-precision%29)))

(event EventDrawHUD
  (params (SizeX :type Integer) (SizeY :type Integer))
  (Variables|Default|SetSize%20X SizeX)
  (Variables|Default|SetSize%20Y SizeY)
  (Utilities|FlowControl|Sequence
    (:then_0
      (if (Variables|Default|GetBlueMode)
        (Class|HUD|DrawMaterialSimple "/Game/Tut_FirstBlood/materials/MAT_HUD.MAT_HUD" 0.0 0.0 (Math|Conversions|ToFloat(Integer) (Variables|Default|GetSize%20X)) (Math|Conversions|ToFloat(Integer) (Variables|Default|GetSize%20Y)) 1.0 false)
        (elif (Variables|Default|GetGreenMode)
          (Class|HUD|DrawMaterialSimple "/Game/Tut_FirstBlood/materials/MAT_HUD_2.MAT_HUD_2" 0.0 0.0 (Math|Conversions|ToFloat(Integer) (Variables|Default|GetSize%20X)) (Math|Conversions|ToFloat(Integer) (Variables|Default|GetSize%20Y)) 1.0 false)
          (elif (Variables|Default|GetRedMode)
            (Class|HUD|DrawMaterialSimple "/Game/Tut_FirstBlood/materials/MAT_HUD_3.MAT_HUD_3" 0.0 0.0 (Math|Conversions|ToFloat(Integer) (Variables|Default|GetSize%20X)) (Math|Conversions|ToFloat(Integer) (Variables|Default|GetSize%20Y)) 1.0 false)
            (else
              (Variables|Default|SetBlueMode true))))))
    (:then_1
      (Class|HUD|DrawMaterialSimple "/Game/Tut_FirstBlood/materials/MAT_COIN.MAT_COIN" (- (Math|Conversions|ToFloat(Integer) (Variables|Default|GetSize%20X)) 2.5e+02) 1e+02 1e+02 1e+02 1.0 false)
      (HUD|DrawText "x" "(R=1.000000,G=1.000000,B=1.000000,A=1.000000)" (- (Math|Conversions|ToFloat(Integer) (Variables|Default|GetSize%20X)) 1.5e+02) 1.2e+02 "/Engine/EngineFonts/RobotoDistanceField.RobotoDistanceField" 2.5 false)
      (bind _asside_scroller_character (Utilities|Casting|CastToSideScrollerCharacter (Game|GetPlayerCharacter 0)))
      (HUD|DrawText (Utilities|String|ToString(Integer) (Variables|/Game/SideScrollerBP/Blueprints/SideScrollerCharacter.SideScrollerCharacter_C|Getcoins _asside_scroller_character)) "(R=1.000000,G=1.000000,B=1.000000,A=1.000000)" (- (Math|Conversions|ToFloat(Integer) (Variables|Default|GetSize%20X)) 1.1e+02) 1.2e+02 "/Engine/EngineFonts/RobotoDistanceField.RobotoDistanceField" 2.5 false))))

(fn ConstructionScript)